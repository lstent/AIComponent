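; AI controller for birds that runs their behavior tree and tells it when it is flocking time.
; On BeginPlay it starts BP_BirdBehaviorTree and caches the BirdsGameInstance.
; Every tick it sets the FlockTime blackboard bool to true while the game instance's SunHeight lies within a band around the horizon, otherwise false.
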(event EventBeginPlay
  (AI|RunBehaviorTree "/Game/Birds/BP_BirdBehaviorTree.BP_BirdBehaviorTree")
  (bind _asbirds_game_instance (Utilities|Casting|CastToBirdsGameInstance (Game|GetGameInstance)))
  (Variables|Default|SetGameInstanceRef _asbirds_game_instance))

(event EventTick
  (params (DeltaSeconds :type Float%20%28single-precision%29))
  (bind _returnvalue (Utilities|Name|MakeLiteralName "FlockTime"))
  (bind _self self)
  (bind _gameinstanceref (Variables|Default|GetGameInstanceRef))
  (bind _returnvalue_2 (AI|GetBlackboard _self))
  (bind _sunheight (Variables|/Game/FirstPersonBP/Blueprints/BirdsGameInstance.BirdsGameInstance_C|GetSunHeight _gameinstanceref))
  (if (and (< _sunheight 6e+01) (> _sunheight -3e+01))
    (AI|Components|Blackboard|SetValueasBool _returnvalue_2 _returnvalue true)
    (else
      (AI|Components|Blackboard|SetValueasBool _returnvalue_2 _returnvalue false))))

(fn ConstructionScript)