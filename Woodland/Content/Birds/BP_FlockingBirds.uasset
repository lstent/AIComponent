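; Bird flock spawner that, on BeginPlay, spawns BP_Bird AI pawns with BP_BirdBehaviorTree at random horizontal offsets within BirdSpawnRadius at a fixed height.
; An older static-mesh boids-style simulation remains but is disconnected, with Tick empty.
; That unused logic averages nearby bird positions to pick bounded wander destinations, then interpolates rotation at randomized turn speeds, moves birds forward and nudges rotation when neighbors get too close.
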(event Custom|UpdateBirdLocations&Destinations
  (Utilities|FlowControl|Sequence
    (:then_0
      (for (_array_element _array_index) (Variables|Default|GetBirds)
        (CallFunction|GetNearbyBirds&TheirDestinations _array_element _array_index))
      ;[1 1 1] Set everyones turn speed
      (Utilities|FlowControl|Gate true) ; enters at Open
    )
    (:then_1
      (Variables|Default|SetUpDownNeither (Math|Random|RandomInteger 3)))))

(event EventBeginPlay
  (bind _birdspawnradius (Variables|Default|GetBirdSpawnRadius))
  (bind _returnvalue (* _birdspawnradius -1.0))
  (for _index (range 1 (Variables|Default|GetNumberOfBirds))
    (AI|SpawnAIFromClass "/Game/Birds/BP_Bird.BP_Bird_C" "/Game/Birds/BP_BirdBehaviorTree.BP_BirdBehaviorTree" (Math|Vector|MakeVector (Math|Random|RandomFloatinRange _returnvalue _birdspawnradius) (Math|Random|RandomFloatinRange _returnvalue _birdspawnradius) 3e+03) "0, 0, 0" false)))

(event EventTick
  (params (DeltaSeconds :type Float%20%28single-precision%29)))

(fn ConstructionScript)

(fn GetNearbyBirds&TheirDestinations
  (params (BirdRef :type Scene%20Component%20Object%20Reference) (BirdIndex :type Integer))
  (bind _returnvalue (Transformation|GetWorldLocation BirdRef))
  (Utilities|Array|SetArrayElem (Variables|Default|GetBirdLocations) BirdIndex _returnvalue)
  (Variables|Default|SetBirdAverageLocation (Math|Vector|GetVectorArrayAverage (Variables|Default|GetBirdLocations)))
  (Utilities|Array|Clear (Variables|Default|GetNearbyBirdLocations))
  (Utilities|Array|Clear (Variables|Default|GetNearbyBirdDestinations))
  (for (_array_element _array_index) (Variables|Default|GetBirdLocations)
    (if (< (Math|Vector|VectorLength (- _array_element _returnvalue)) (* (Variables|Default|GetBirdSpawnRadius) (Variables|Default|GetDistanceScale)))
      (Utilities|Array|Add (Variables|Default|GetNearbyBirdLocations) _array_element)
      (Utilities|Array|Add (Variables|Default|GetNearbyBirdDestinations) (Utilities|Array|Get(acopy) (Variables|Default|GetBirdDestinations) _array_index)))))

(fn SetNewDestination
  (bind _returnvalue (Transformation|GetActorLocation))
  (bind _nearbybirdlocations (Variables|Default|GetNearbyBirdLocations))
  (bind _birdspawnradius (Variables|Default|GetBirdSpawnRadius))
  (bind _flocksizekinda (Variables|Default|GetFlockSizeKinda))
  (bind _returnvalue_2 (Math|Vector|GetVectorArrayAverage _nearbybirdlocations))
  (bind _returnvalue_3 (* _birdspawnradius _flocksizekinda))
  (Variables|Default|SetProposedNewDestination (Math|Random|RandomPointinBoundingBox (select (> (Math|Vector|VectorLength (- _returnvalue_2 _returnvalue)) (Variables|Default|GetWanderDistance)) _returnvalue (+ _returnvalue_2 (Utilities|Select :Index (Variables|Default|GetUpDownNeither) :Option%200 "0,0,1000.000000" :Option%201 "0.000000,0.000000,-1000.000000" :Option%202 "0, 0, 0"))) (Math|Vector|MakeVector _returnvalue_3 _returnvalue_3 (* _returnvalue_3 1.0))))
  (return))

(fn SetBirdsDestinationtoProposedNewDestination
  (params (BirdIndex :type Integer))
  (Utilities|Array|SetArrayElem (Variables|Default|GetBirdDestinations) BirdIndex (Variables|Default|GetProposedNewDestination)))

(fn CheckProposedDesinationIsn'ttheSameasAnotherBird
  (bind _array_element (Utilities|Array|ForEachLoopwithBreak (Variables|Default|GetNearbyBirdLocations))
    (:LoopBody
      (if (< (Math|Vector|VectorLength (- _array_element (Variables|Default|GetProposedNewDestination))) 5.0)
        (Variables|Default|SetProposedNewDestination (+ (Variables|Default|GetProposedNewDestination) (Utilities|Select :Index (Math|Random|RandomInteger 3) :Option%200 (Math|Vector|MakeVector (Math|Random|RandomFloatinRange -5.0 5.0) 0.0 0.0) :Option%201 (Math|Vector|MakeVector 0.0 (Math|Random|RandomFloatinRange -5.0 5.0) 0.0) :Option%202 (Math|Vector|MakeVector 0.0 0.0 (Math|Random|RandomFloatinRange -5.0 5.0)))))))
    (:Completed
      (return))))

(fn TurnBirdTowardsDestination
  (params (BirdIndex :type Integer) (BirdRef :type Static%20Mesh%20Component%20Object%20Reference))
  (Transformation|SetWorldRotation BirdRef (Math|Interpolation|RInterpTo (Transformation|GetWorldRotation BirdRef) (Math|Rotator|FindLookatRotation (Transformation|GetWorldLocation BirdRef) (Utilities|Array|Get(acopy) (Variables|Default|GetBirdDestinations) BirdIndex)) (Variables|Default|GetDeltatime) (Variables|Default|GetTurnSpeed)) false false)
  (Math|Random|SetRandomStreamSeed (Variables|Default|GetStream) BirdIndex)
  (return))

(fn MoveBirdForward
  (params (BirdRef :type Scene%20Component%20Object%20Reference))
  (Transformation|AddLocalOffset BirdRef (Math|Vector|MakeVector (* (Variables|Default|GetBaseSpeed) (Variables|Default|GetDeltatime)) 0.0 0.0) false false))

(fn RotateAwayfromOtherBirds
  (params (BirdRef :type Static%20Mesh%20Component%20Object%20Reference))
  (bind _array_element (Utilities|Array|ForEachLoopwithBreak (Variables|Default|GetNearbyBirdLocations) :!label _label)
    (:LoopBody
      (if (< (Math|Vector|VectorLength (- _array_element (Transformation|GetWorldLocation BirdRef))) 2e+01)
        (Transformation|AddLocalRotation BirdRef (Math|Rotator|MakeRotator 0.0 1.0 1.0) false false)
        (goto _label Break)))))