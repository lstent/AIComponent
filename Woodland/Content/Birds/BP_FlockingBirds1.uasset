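; Flock manager actor that spawns BP_Bird AI pawns at altitude and steers them as a loose, wandering flock.
; Randomly delayed updates on Tick refresh shared nearby-bird lists and a random vertical bias.
; Each tick gives every bird a random destination around that neighbor average, or around the manager when it strays beyond WanderDistance.
; Birds interpolate their rotation toward it, move forward (local up at low altitude), and nudge rotation when crowded.
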(event Custom|UpdateBirdLocations&Destinations
  (params (BirdRef :type Pawn%20Object%20Reference) (BirdIndex :type Integer))
  (Utilities|FlowControl|Sequence
    (:then_0
      (CallFunction|GetNearbyBirds&TheirDestinations BirdRef BirdIndex))
    (:then_1
      (Variables|Default|SetUpDownNeither (Math|Random|RandomInteger 3)))))

(event EventBeginPlay
  (bind _birdspawnradius (Variables|Default|GetBirdSpawnRadius))
  (bind _returnvalue (* _birdspawnradius -1.0))
  (for _index (range 1 (Variables|Default|GetNumberOfBirds))
    (bind _returnvalue_2 (AI|SpawnAIFromClass "/Game/Birds/BP_Bird.BP_Bird_C" "/Game/Birds/BP_BirdBehaviorTree.BP_BirdBehaviorTree" (Math|Vector|MakeVector (Math|Random|RandomFloatinRange _returnvalue _birdspawnradius) (Math|Random|RandomFloatinRange _returnvalue _birdspawnradius) 6e+03) "0, 0, 0" true))
    (bind _returnvalue_3 (Utilities|Array|AddUnique (Variables|Default|GetBirds) _returnvalue_2))
    (if (== _returnvalue_3 0)
      (Rendering|SetActorHiddenInGame _returnvalue_2 true))
    (Utilities|Array|Add (Variables|Default|GetBirdDestinations) (+ (Transformation|GetActorLocation _returnvalue_2) (* (Transformation|GetActorForwardVector _returnvalue_2) 2e+01)))
    (Utilities|Array|Add (Variables|Default|GetBirdLocations) (Transformation|GetActorLocation _returnvalue_2))))

(event EventTick
  (params (DeltaSeconds :type Float%20%28single-precision%29))
  (Variables|Default|SetDeltatime DeltaSeconds)
  (Utilities|FlowControl|Sequence
    (:then_0
      (for _array_element (Variables|Default|GetBirds)
        (Utilities|FlowControl|Delay (Math|Random|RandomFloatinRange 0.1 2.0))
        (for (_array_element_2 _array_index) (Variables|Default|GetBirds)
          (Utilities|FlowControl|Delay (Math|Random|RandomFloatinRange 0.1 (Variables|Default|GetInterval)))
          (CallFunction|UpdateBirdLocations&Destinations _array_element_2 _array_index))
        (goto _label Open)))
    (:then_1
      (for (_array_element_3 _array_index_2) (Variables|Default|GetBirds)
        (Utilities|FlowControl|Sequence
          (:then_0
            (CallFunction|SetNewDestination)
            (CallFunction|CheckProposedDesinationIsn'ttheSameasAnotherBird)
            (CallFunction|SetBirdsDestinationtoProposedNewDestination _array_index_2))
          (:then_1
            (CallFunction|TurnBirdTowardsDestination _array_index_2 _array_element_3)
            ;[1 1 1] Set everyones turn speed
            (Utilities|FlowControl|Gate true :!label _label
              (:Exit
                (Variables|Default|SetTurnSpeed (* (Math|Random|RandomFloatinRange 0.0 1.0) (Math|Random|RandomFloatinRangefromStream 0.5 2.0 (Variables|Default|GetStream)))))))
          (:then_2
            (CallFunction|MoveBirdForward _array_element_3))
          (:then_3
            (CallFunction|RotateAwayfromOtherBirds _array_element_3))))
      (Utilities|FlowControl|Gate true) ; enters at Close
    )))

(fn ConstructionScript)

(fn GetNearbyBirds&TheirDestinations
  (params (BirdRef :type Pawn%20Object%20Reference) (BirdIndex :type Integer))
  (bind _returnvalue (Transformation|GetActorLocation BirdRef))
  (Utilities|Array|SetArrayElem (Variables|Default|GetBirdLocations) BirdIndex _returnvalue)
  (Variables|Default|SetBirdAverageLocation (Math|Vector|GetVectorArrayAverage (Variables|Default|GetBirdLocations)))
  (Utilities|Array|Clear (Variables|Default|GetNearbyBirdLocations))
  (Utilities|Array|Clear (Variables|Default|GetNearbyBirdDestinations))
  (for (_array_element _array_index) (Variables|Default|GetBirdLocations)
    (if (< (Math|Vector|VectorLength (- _array_element _returnvalue)) (* (Variables|Default|GetBirdSpawnRadius) (Variables|Default|GetDistanceScale)))
      (Utilities|Array|Add (Variables|Default|GetNearbyBirdLocations) _array_element)
      (Utilities|Array|Add (Variables|Default|GetNearbyBirdDestinations) (Utilities|Array|Get(acopy) (Variables|Default|GetBirdDestinations) _array_index)))))

(fn SetNewDestination
  (bind _returnvalue (Transformation|GetActorLocation))
  (bind _nearbybirdlocations (Variables|Default|GetNearbyBirdLocations))
  (bind _birdspawnradius (Variables|Default|GetBirdSpawnRadius))
  (bind _flocksizekinda (Variables|Default|GetFlockSizeKinda))
  (bind _returnvalue_2 (Math|Vector|GetVectorArrayAverage _nearbybirdlocations))
  (bind _returnvalue_3 (* _birdspawnradius _flocksizekinda))
  (Variables|Default|SetProposedNewDestination (Math|Random|RandomPointinBoundingBox (select (> (Math|Vector|VectorLength (- _returnvalue_2 _returnvalue)) (Variables|Default|GetWanderDistance)) _returnvalue (+ _returnvalue_2 (Utilities|Select :Index (Variables|Default|GetUpDownNeither) :Option%200 "0,0,1000.000000" :Option%201 "0.000000,0.000000,-1000.000000" :Option%202 "0, 0, 0"))) (Math|Vector|MakeVector _returnvalue_3 _returnvalue_3 (* _returnvalue_3 1.0))))
  (return))

(fn SetBirdsDestinationtoProposedNewDestination
  (params (BirdIndex :type Integer))
  (Utilities|Array|SetArrayElem (Variables|Default|GetBirdDestinations) BirdIndex (Variables|Default|GetProposedNewDestination)))

(fn CheckProposedDesinationIsn'ttheSameasAnotherBird
  (bind _array_element (Utilities|Array|ForEachLoopwithBreak (Variables|Default|GetNearbyBirdLocations))
    (:LoopBody
      (if (< (Math|Vector|VectorLength (- _array_element (Variables|Default|GetProposedNewDestination))) 5.0)
        (Variables|Default|SetProposedNewDestination (+ (Variables|Default|GetProposedNewDestination) (Utilities|Select :Index (Math|Random|RandomInteger 3) :Option%200 (Math|Vector|MakeVector (Math|Random|RandomFloatinRange -5.0 5.0) 0.0 0.0) :Option%201 (Math|Vector|MakeVector 0.0 (Math|Random|RandomFloatinRange -5.0 5.0) 0.0) :Option%202 (Math|Vector|MakeVector 0.0 0.0 (Math|Random|RandomFloatinRange -5.0 5.0)))))))
    (:Completed
      (return))))

(fn TurnBirdTowardsDestination
  (params (BirdIndex :type Integer) (BirdRef :type Pawn%20Object%20Reference))
  (Transformation|SetActorRotation BirdRef (Math|Interpolation|RInterpTo (Transformation|GetActorRotation BirdRef) (Math|Rotator|FindLookatRotation (Transformation|GetActorLocation BirdRef) (Utilities|Array|Get(acopy) (Variables|Default|GetBirdDestinations) BirdIndex)) (Variables|Default|GetDeltatime) (Variables|Default|GetTurnSpeed)))
  (Math|Random|SetRandomStreamSeed (Variables|Default|GetStream) BirdIndex)
  (return))

(fn MoveBirdForward
  (params (BirdRef :type Pawn%20Object%20Reference))
  (bind _basespeed (Variables|Default|GetBaseSpeed))
  (bind _deltatime (Variables|Default|GetDeltatime))
  (bind _returnvalue (* _basespeed _deltatime))
  (if (<= (.z (Transformation|GetActorLocation BirdRef)) 2e+03)
    (Transformation|AddActorLocalOffset BirdRef (Math|Vector|MakeVector 0.0 0.0 _returnvalue) false false)
    (else
      (Transformation|AddActorLocalOffset BirdRef (Math|Vector|MakeVector _returnvalue 0.0 0.0) false false))))

(fn RotateAwayfromOtherBirds
  (params (BirdRef :type Pawn%20Object%20Reference))
  (bind _array_element (Utilities|Array|ForEachLoopwithBreak (Variables|Default|GetNearbyBirdLocations) :!label _label)
    (:LoopBody
      (if (< (Math|Vector|VectorLength (- _array_element (Transformation|GetActorLocation BirdRef))) 2e+01)
        (Transformation|AddActorLocalRotation BirdRef (Math|Rotator|MakeRotator 0.0 1.0 1.0) false false)
        (goto _label Break)))))