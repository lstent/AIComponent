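; BP_FlyingPig is a grid-bound pig actor that snaps to the nearest BP_Grid tile when play begins.
; BeginPlay caches the grid and first-person player, then linearly searches StructTiles for the closest WorldLocation, storing that index and teleporting there.
; MoveAlongPath is unfinished: it stores the path and clears the grid's spline, but its loop is empty, so no movement occurs.
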(event Custom|MoveAlongPath
  (params (Path :type Array%20of%20Vectors))
  (Variables|Default|SetPath Path)
  (Spline|ClearSplinePoints (Variables|/Game/Geometry/BP_Grid.BP_Grid_C|GetSpline (Variables|References|GetGridRef)) true)
  (for _array_element (Variables|Default|GetPath)
    _))

(event EventBeginPlay
  (bind _outactors (Actor|GetAllActorsOfClass "/Game/Geometry/BP_Grid.BP_Grid_C"))
  (Variables|References|SetGridRef (Utilities|Array|Get(acopy) _outactors))
  (bind _asfirst_person_character (Utilities|Casting|CastToFirstPersonCharacter (Game|GetPlayerCharacter 0))
    (:then
      (Variables|References|SetPlayerRef _asfirst_person_character))
    (:CastFailed
      _))
  (CallFunction|SetGridIndex&SnaptoLocation))

(event EventTick
  (params (DeltaSeconds :type Float%20%28single-precision%29)))

(fn ConstructionScript)

(fn SetGridIndex&SnaptoLocation
  (LocalVariables|SetClosestDistance 9999999.0)
  (bind _keys (Utilities|Map|Keys (Variables|/Game/Geometry/BP_Grid.BP_Grid_C|GetStructTiles (Variables|References|GetGridRef))))
  (for _array_element _keys
    (if (< (Math|Vector|VectorLength (- (.worldlocation (.Value (Utilities|Map|Find (Variables|/Game/Geometry/BP_Grid.BP_Grid_C|GetStructTiles (Variables|References|GetGridRef)) _array_element))) (Transformation|GetActorLocation self))) (LocalVariables|GetClosestDistance))
      (LocalVariables|SetClosestDistance (Math|Vector|VectorLength (- (.worldlocation (.Value (Utilities|Map|Find (Variables|/Game/Geometry/BP_Grid.BP_Grid_C|GetStructTiles (Variables|References|GetGridRef)) _array_element))) (Transformation|GetActorLocation self))))
      (LocalVariables|SetClosestIndex _array_element)))
  (Variables|Default|SetGridIndex (LocalVariables|GetClosestIndex))
  (Transformation|SetActorLocation (.worldlocation (.Value (Utilities|Map|Find (Variables|/Game/Geometry/BP_Grid.BP_Grid_C|GetStructTiles (Variables|References|GetGridRef)) (LocalVariables|GetClosestIndex)))) false true))