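; BP_Grid is a 3D navigation grid that supplies A* pathfinding, likely for BP_FlyingPig, which it references at BeginPlay along with the player.
; The construction script sphere-traces each cell in the world, storing it as FreeSpace or Danger in a map keyed by grid index.
; FindPathToTarget searches non-Danger cells among 14 neighbour offsets, using tile costs and a Manhattan heuristic, then retraces parent links into a path.
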(event EventBeginPlay
  ;[1 1 1] References
  (Grid|SetReferences))

(fn ConstructionScript
  (Rendering|Debug|FlushPersistentDebugLines)
  (Variables|Grid|SetGridLocation (Transformation|GetWorldLocation (Variables|Default|GetScene)))
  (Grid|GenetateMapDatafromWorld))

(fn GridBottomLeft
  (return (- (- (- (Variables|Grid|GetGridLocation) (* (Math|Vector|GetRightVector (Variables|Default|GetScene)) (.x (Variables|Grid|GetGridSizeWorld)))) (* (Math|Vector|GetForwardVector (Variables|Default|GetScene)) (.y (Variables|Grid|GetGridSizeWorld)))) (- (* (Math|Vector|GetUpVector (Variables|Default|GetScene)) (.z (Variables|Grid|GetGridSizeWorld))) (Variables|Grid|GetGridLocation)))))

(fn GridTileNumber
  (bind _gridsizeworld (Variables|Grid|GetGridSizeWorld))
  (bind _makesuretilenumberstartsatzero (LocalVariables|GetMakeSureTileNumberStartsAtZero))
  (bind _tilesize (Variables|Grid|GetTileSize))
  (bind _returnvalue (/ _gridsizeworld _tilesize))
  (return (- (Math|Float|Round (.x _returnvalue)) _makesuretilenumberstartsatzero) (- (Math|Float|Round (.y _returnvalue)) _makesuretilenumberstartsatzero) (- (Math|Float|Round (.z _returnvalue)) _makesuretilenumberstartsatzero)))

(fn DrawTile
  (bind _keys (Utilities|Map|Keys (Variables|Grid|GetStructTiles)))
  (for _array_element _keys
    (Debug|DrawDebugPlane (.groundtype (.Value (Utilities|Map|Find (Variables|Grid|GetStructTiles) _array_element))) (.worldlocation (.Value (Utilities|Map|Find (Variables|Grid|GetStructTiles) _array_element))))))

(fn SphereTrace
  (params (Location :type Vector) (TraceChannel :type ETraceTypeQuery%20Enum :default "TraceTypeQuery1"))
  (bind _returnvalue (Collision|SphereTraceByChannel (+ Location (LocalVariables|GetStartCan'tBeTheSameAsEnd)) Location (- (Variables|Grid|GetTileSize) (Variables|Grid|GetTileSizeMinus)) TraceChannel false 0 "Persistent" true "(R=1.000000,G=0.000000,B=0.000000,A=1.000000)" "(R=0.000000,G=1.000000,B=0.000000,A=1.000000)" 2e+01))
  (return _returnvalue))

(fn GenetateMapDatafromWorld
  (bind (_gridtilenumberx _gridtilenumbery _gridtilenumberz) (Grid|GridTileNumber))
  (for _index (range (LocalVariables|GetStartIndex) _gridtilenumberx)
    (Variables|Grid|SetTileX _index)
    (for _index_2 (range (LocalVariables|GetStartIndex) _gridtilenumbery)
      (Variables|Grid|SetTileY _index_2)
      (for _index_3 (range (LocalVariables|GetStartIndex) _gridtilenumberz)
        (Variables|Grid|SetTileZ _index_3)
        (LocalVariables|SetTilePosition (Grid|CalculateTilePosition))
        (if (Grid|SphereTrace (LocalVariables|GetTilePosition) "TraceTypeQuery4")
          (Utilities|Map|Add (Variables|Grid|GetStructTiles) (Math|Vector|MakeVector (Math|Conversions|ToFloat(Integer) (Variables|Grid|GetTileX)) (Math|Conversions|ToFloat(Integer) (Variables|Grid|GetTileY)) (Math|Conversions|ToFloat(Integer) (Variables|Grid|GetTileZ))) (Utilities|Struct|MakeStruct_Tiles 0 "NewEnumerator1" (LocalVariables|GetTilePosition) (Math|Vector|MakeVector (Math|Conversions|ToFloat(Integer) (Variables|Grid|GetTileX)) (Math|Conversions|ToFloat(Integer) (Variables|Grid|GetTileY)) (Math|Conversions|ToFloat(Integer) (Variables|Grid|GetTileZ))) (Grid|GetTileCost (Math|Vector|MakeVector (Math|Conversions|ToFloat(Integer) (Variables|Grid|GetTileX)) (Math|Conversions|ToFloat(Integer) (Variables|Grid|GetTileY)) (Math|Conversions|ToFloat(Integer) (Variables|Grid|GetTileZ)))) 0 0 0 "0.000000,0.000000,0.000000"))
          (else
            (Utilities|Map|Add (Variables|Grid|GetStructTiles) (Math|Vector|MakeVector (Math|Conversions|ToFloat(Integer) (Variables|Grid|GetTileX)) (Math|Conversions|ToFloat(Integer) (Variables|Grid|GetTileY)) (Math|Conversions|ToFloat(Integer) (Variables|Grid|GetTileZ))) (Utilities|Struct|MakeStruct_Tiles 0 "NewEnumerator2" (LocalVariables|GetTilePosition) (Math|Vector|MakeVector (Math|Conversions|ToFloat(Integer) (Variables|Grid|GetTileX)) (Math|Conversions|ToFloat(Integer) (Variables|Grid|GetTileY)) (Math|Conversions|ToFloat(Integer) (Variables|Grid|GetTileZ))) (Grid|GetTileCost (Math|Vector|MakeVector (Math|Conversions|ToFloat(Integer) (Variables|Grid|GetTileX)) (Math|Conversions|ToFloat(Integer) (Variables|Grid|GetTileY)) (Math|Conversions|ToFloat(Integer) (Variables|Grid|GetTileZ)))) 0 0 0 "0.000000,0.000000,0.000000"))))))))

(fn DrawDebugPlane
  (params (GroundType :type Enum_GroundTypes%20Enum :default "NewEnumerator2") (Location :type Vector))
  (switch Utilities|FlowControl|Switch|SwitchonEnum_GroundTypes GroundType
    (:NewEnumerator2
      (Variables|Debug|SetTileColour "(R=0.958333,G=0.958333,B=0.958333,A=1.000000)"))
    (:NewEnumerator1
      (Variables|Debug|SetTileColour "(R=0.765625,G=0.000000,B=0.000000,A=1.000000)")))
  (Class|KismetSystemLibrary|DrawDebugPlane (Utilities|Struct|MakePlane (.Z (Math|Vector|BreakVector Location)) 0.0 0.0 1.0) Location (- (Variables|Grid|GetTileSize) (Variables|Grid|GetTileSizeMinus)) (Variables|Debug|GetTileColour) 1e+05))

(fn GetTileCost
  (params (GridIndex :type Vector))
  (switch Utilities|FlowControl|Switch|SwitchonEnum_GroundTypes (.groundtype (.Value (Utilities|Map|Find (Variables|Grid|GetStructTiles) GridIndex)))
    (:NewEnumerator2
      (LocalVariables|SetCost (LocalVariables|GetFreeSpaceCost)))
    (:NewEnumerator1
      (LocalVariables|SetCost (LocalVariables|GetBlockedSpaceCost))))
  (return (LocalVariables|GetCost)))

(fn GetTileNeighbors
  (params (GridIndex :type Vector))
  (Utilities|Array|Clear (LocalVariables|GetPossibleNeighbors))
  (bind _output_get (LocalVariables|SetPossibleNeighbors (Utilities|Array|MakeArray (LocalVariables|GetBehind) (LocalVariables|GetRight) (LocalVariables|GetUp) (LocalVariables|GetDown) (LocalVariables|GetLeft) (LocalVariables|GetFront) (LocalVariables|GetBehindRight) (LocalVariables|GetBehindUp) (LocalVariables|GetRightUp) (LocalVariables|GetBehindRightUp) (LocalVariables|GetFrontLeft) (LocalVariables|GetLeftDown) (LocalVariables|GetFrontDown) (LocalVariables|GetFrontLeftDown))))
  (for _array_element _output_get
    (if (.ReturnValue (Utilities|Map|Find (Variables|Grid|GetStructTiles) (+ _array_element GridIndex)))
      (if (Utilities|Enum|NotEqual(Enum) (.groundtype (.Value (Utilities|Map|Find (Variables|Grid|GetStructTiles) (+ _array_element GridIndex)))) "NewEnumerator1")
        (Utilities|Array|AddUnique (LocalVariables|GetOutNeighbors) (+ _array_element GridIndex)))))
  (return (LocalVariables|GetOutNeighbors)))

(fn GetEstimatedCosttoTarget
  (params (CurrentIndex :type Vector) (TargetTile :type Vector))
  (bind _returnvalue (- CurrentIndex TargetTile))
  (return (Math|Float|Round (+ (Math|Float|Absolute(Float) (.x _returnvalue)) (Math|Float|Absolute(Float) (.y _returnvalue)) (Math|Float|Absolute(Float) (.z _returnvalue))))))

(fn FindPathtoTarget
  (params (StartTile :type Vector) (EndTile :type Vector))
  (bind _structtiles (Variables|Grid|GetStructTiles))
  (bind _structtiles_2 (Variables|Grid|GetStructTiles))
  (bind _structtiles_3 (Variables|Grid|GetStructTiles))
  (LocalVariables|SetStartTileL StartTile)
  (LocalVariables|SetTargetTileL EndTile)
  (if (and (Utilities|Enum|NotEqual(Enum) (.groundtype (.Value (Utilities|Map|Find (Variables|Grid|GetStructTiles) (LocalVariables|GetTargetTileL)))) "NewEnumerator1") (.ReturnValue (Utilities|Map|Find (Variables|Grid|GetStructTiles) (LocalVariables|GetTargetTileL))))
    (Utilities|FlowControl|Sequence
      (:then_0
        ;[1 1 1] Default values
        (bind _keys (Utilities|Map|Keys (Variables|Grid|GetStructTiles)))
        (for _array_element _keys
          (Utilities|Map|Add _structtiles_3 _array_element (Utilities|Struct|MakeStruct_Tiles (.actorusingpathfinding (.Value (Utilities|Map|Find _structtiles_3 _array_element))) (.groundtype (.Value (Utilities|Map|Find _structtiles_3 _array_element))) (.worldlocation (.Value (Utilities|Map|Find _structtiles_3 _array_element))) (.gridindex (.Value (Utilities|Map|Find _structtiles_3 _array_element))) (.tilecost (.Value (Utilities|Map|Find _structtiles_3 _array_element))) 999 999 999 "0.000000,0.000000,0.000000")))
        (Utilities|Map|Add _structtiles (LocalVariables|GetStartTileL) (Utilities|Struct|MakeStruct_Tiles (.actorusingpathfinding (.Value (Utilities|Map|Find _structtiles (LocalVariables|GetStartTileL)))) (.groundtype (.Value (Utilities|Map|Find _structtiles (LocalVariables|GetStartTileL)))) (.worldlocation (.Value (Utilities|Map|Find _structtiles (LocalVariables|GetStartTileL)))) (.gridindex (.Value (Utilities|Map|Find _structtiles (LocalVariables|GetStartTileL)))) (.tilecost (.Value (Utilities|Map|Find _structtiles (LocalVariables|GetStartTileL)))) (PathFinding|GetEstimatedCosttoTarget (LocalVariables|GetStartTileL) (LocalVariables|GetTargetTileL)) 0 (PathFinding|GetEstimatedCosttoTarget (LocalVariables|GetStartTileL) (LocalVariables|GetTargetTileL)) "0.000000,0.000000,0.000000")))
      (:then_1
        (bind _output_get (LocalVariables|SetCurrentTile (LocalVariables|GetStartTileL)))
        (Utilities|Array|AddUnique (LocalVariables|GetOpenSet) _output_get)
        (while (> (Utilities|Array|Length (LocalVariables|GetOpenSet)) (LocalVariables|GetZero))
          (LocalVariables|SetOpenSetCheapest (Utilities|Array|Get(acopy) (LocalVariables|GetOpenSet)))
          (for _array_element_2 (LocalVariables|GetOpenSet)
            (if (< (.finalcost (.Value (Utilities|Map|Find _structtiles_2 _array_element_2))) (.finalcost (.Value (Utilities|Map|Find _structtiles_2 (LocalVariables|GetOpenSetCheapest)))))
              (LocalVariables|SetOpenSetCheapest _array_element_2 :!label _label)
              (elif (== (.finalcost (.Value (Utilities|Map|Find _structtiles_2 _array_element_2))) (.finalcost (.Value (Utilities|Map|Find _structtiles_2 (LocalVariables|GetOpenSetCheapest)))))
                (if (< (.estimatecosttotarget (.Value (Utilities|Map|Find _structtiles_2 _array_element_2))) (.estimatecosttotarget (.Value (Utilities|Map|Find _structtiles_2 (LocalVariables|GetOpenSetCheapest)))))
                  (goto _label)))))
          ;[1 1 1] Go through neighbor array & find cheapest path
          (LocalVariables|SetCurrentTile (LocalVariables|GetOpenSetCheapest))
          (Utilities|Array|RemoveItem (LocalVariables|GetOpenSet) (LocalVariables|GetCurrentTile))
          (Utilities|Array|AddUnique (LocalVariables|GetClosedSet) (LocalVariables|GetCurrentTile))
          (if (not (Math|Vector|Equal(Vector) (LocalVariables|GetPreviousEndTile) (LocalVariables|GetTargetTileL) (LocalVariables|GetThreshold)))
            (LocalVariables|SetPreviousEndTile (LocalVariables|GetCurrentTile))
            (for _array_element_3 (PathFinding|GetTileNeighbors (LocalVariables|GetCurrentTile))
              (LocalVariables|SetCurrentNeighbour _array_element_3)
              (if (not (Utilities|Array|ContainsItem (LocalVariables|GetClosedSet) (LocalVariables|GetCurrentNeighbour)))
                (LocalVariables|SetCurrentNeighborCostFromStart (+ (.costfromstart (.Value (Utilities|Map|Find (Variables|Grid|GetStructTiles) (LocalVariables|GetCurrentTile)))) (.tilecost (.Value (Utilities|Map|Find (Variables|Grid|GetStructTiles) (LocalVariables|GetCurrentNeighbour))))))
                (if (not (Utilities|Array|ContainsItem (LocalVariables|GetOpenSet) (LocalVariables|GetCurrentNeighbour)))
                  (Utilities|Array|AddUnique (LocalVariables|GetOpenSet) (LocalVariables|GetCurrentNeighbour))
                  (Utilities|Map|Add (Variables|Grid|GetStructTiles) (LocalVariables|GetCurrentNeighbour) (Utilities|Struct|MakeStruct_Tiles (.actorusingpathfinding (.Value (Utilities|Map|Find (Variables|Grid|GetStructTiles) (LocalVariables|GetCurrentNeighbour)))) (.groundtype (.Value (Utilities|Map|Find (Variables|Grid|GetStructTiles) (LocalVariables|GetCurrentNeighbour)))) (.worldlocation (.Value (Utilities|Map|Find (Variables|Grid|GetStructTiles) (LocalVariables|GetCurrentNeighbour)))) (.gridindex (.Value (Utilities|Map|Find (Variables|Grid|GetStructTiles) (LocalVariables|GetCurrentNeighbour)))) (.tilecost (.Value (Utilities|Map|Find (Variables|Grid|GetStructTiles) (LocalVariables|GetCurrentNeighbour)))) (+ (LocalVariables|GetCurrentNeighborCostFromStart) (PathFinding|GetEstimatedCosttoTarget (LocalVariables|GetCurrentNeighbour) (LocalVariables|GetTargetTileL))) (LocalVariables|GetCurrentNeighborCostFromStart) (PathFinding|GetEstimatedCosttoTarget (LocalVariables|GetCurrentNeighbour) (LocalVariables|GetTargetTileL)) (LocalVariables|GetCurrentTile)) :!label _label_2)
                  (if (Math|Vector|Equal(Vector) (LocalVariables|GetCurrentNeighbour) (LocalVariables|GetTargetTileL) (LocalVariables|GetThreshold))
                    (Variables|Grid|SetPath (PathFinding|RetracePath (LocalVariables|GetTargetTileL) (LocalVariables|GetStartTileL)))
                    (return))
                  (elif (< (LocalVariables|GetCurrentNeighborCostFromStart) (.costfromstart (.Value (Utilities|Map|Find (Variables|Grid|GetStructTiles) (LocalVariables|GetCurrentNeighbour)))))
                    (goto _label_2)))))))
        ;[1 1 1] Fail
        (return)))))

(fn RetracePath
  (params (StartTileEnd :type Vector) (TargetTileStart :type Vector))
  (LocalVariables|SetCurrentTile StartTileEnd)
  (while (Math|Vector|NotEqual(Vector) (LocalVariables|GetCurrentTile) TargetTileStart (LocalVariables|GetThreshold))
    (Utilities|Array|AddUnique (LocalVariables|GetInvertedPath) (LocalVariables|GetCurrentTile))
    (LocalVariables|SetCurrentTile (.previoustile (.Value (Utilities|Map|Find (Variables|Grid|GetStructTiles) (LocalVariables|GetCurrentTile))))))
  (bind _arrayelement (Utilities|Array|ReverseforEachLoop (LocalVariables|GetInvertedPath))
    (:LoopBody
      (Utilities|Array|AddUnique (LocalVariables|GetOutPath) _arrayelement))
    (:Completed
      (return (LocalVariables|GetOutPath)))))

(fn SetReferences
  (bind _outactors (Actor|GetAllActorsOfClass "/Game/FlyingPigs/BP_FlyingPig.BP_FlyingPig_C"))
  (Variables|References|SetFlyingPigRef (Utilities|Array|Get(acopy) _outactors))
  (bind _asfirst_person_character (Utilities|Casting|CastToFirstPersonCharacter (Game|GetPlayerCharacter 0)))
  (Variables|References|SetPlayerRef _asfirst_person_character))

(fn CalculateTilePosition
  (bind _tilesize (Variables|Grid|GetTileSize))
  (bind _tilesize_2 (Variables|Grid|GetTileSize))
  (bind _tilesize_3 (Variables|Grid|GetTileSize))
  (return (+ (Grid|GridBottomLeft) (* (Math|Vector|GetRightVector (Variables|Default|GetScene)) (+ (* (Variables|Grid|GetTileX) (* _tilesize_3 (LocalVariables|GetGridOffset))) _tilesize_3)) (* (Math|Vector|GetForwardVector (Variables|Default|GetScene)) (+ (* (Variables|Grid|GetTileY) (* _tilesize (LocalVariables|GetGridOffset))) _tilesize)) (* (Math|Vector|GetUpVector (Variables|Default|GetScene)) (+ (* (Variables|Grid|GetTileZ) (* _tilesize_2 (LocalVariables|GetGridOffset))) _tilesize_2)))))