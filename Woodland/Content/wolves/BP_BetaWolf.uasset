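; BP_BetaWolf is a follower wolf that moves toward the pack's alpha.
; On BeginPlay it caches the first BP_AlphaWolf found in the level.
; Each Tick, when not already moving, it starts an AI MoveTo targeting that alpha, using a Moving flag that resets on success or failure so a new move can begin.
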(event EventBeginPlay
  (bind _outactors (Actor|GetAllActorsOfClass "/Game/wolves/BP_AlphaWolf.BP_AlphaWolf_C"))
  (Variables|Default|SetAlphaWolfRef (Utilities|Array|Get(acopy) _outactors)))

(event Collision|EventActorBeginOverlap
  (params (OtherActor :type Actor%20Object%20Reference)))

(event EventTick
  (params (DeltaSeconds :type Float%20%28single-precision%29))
  (bind _alphawolfref (Variables|Default|GetAlphaWolfRef))
  (if (not (Variables|Default|GetMoving))
    (AI|AIMoveTo self (Transformation|GetActorLocation _alphawolfref) _alphawolfref 5.0 false
      (:then
        (Variables|Default|SetMoving true))
      (:OnSuccess
        (Variables|Default|SetMoving false :!label _label))
      (:OnFail
        (goto _label)))))

(fn ConstructionScript)